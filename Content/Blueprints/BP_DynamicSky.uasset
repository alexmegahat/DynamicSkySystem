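; Dynamic sky actor that sets up a day or night sky from a TimeOfDay value, entirely in the Construction Script.
; It creates a dynamic material on the sky sphere, then maps time to sun and moon light pitch around dawn and dusk.
; A padded dawn-to-dusk check toggles the lights and switches Sky Atmosphere scattering.
; At night it also applies moonlight settings and drives the material's star and moon parameters.
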(event EventBeginPlay)

(event Collision|EventActorBeginOverlap
  (params (OtherActor :type Actor%20Object%20Reference)))

(event EventTick
  (params (DeltaSeconds :type Float%20%28single-precision%29)))

(fn ConstructionScript
  (bind _is_dynmi_skyspherevalid (01-BasicSettings|InitSkySphereMaterial))
  (if _is_dynmi_skyspherevalid
    (Utilities|FlowControl|Sequence
      (:then_1
        (01-BasicSettings|HandleSunMoonRotation))
      (:then_2
        (01-BasicSettings|HandleSunMoonVisibility))
      (:then_3
        (02-NightSettings|HandleNightSettings)))))

(fn InitSkySphereMaterial
  (bind _returnvalue (Rendering|Material|CreateDynamicMaterialInstance (Variables|Default|GetSM_SkySphere) 0 (Variables|03-NightSettings|GetNightSky%20Material) "None" :!class /Script/Engine.PrimitiveComponent))
  (bind _output_get (Variables|Default|SetCreated_DynMI_SkySphere _returnvalue))
  (return (Utilities|IsValid _output_get)))

(fn HandleSunMoonVisibility
  (Rendering|SetVisibility (Variables|Default|GetSunDirectionalLight) (Utilities|IsDayTime) false)
  (Rendering|SetVisibility (Variables|Default|GetMoonDirectionalLight) (Utilities|IsNightTime) false))

(fn HandleSunMoonRotation
  ;[0.15 0.15 0.15 0.5] Handle Sun rotation between Dawn and Dusk
  (Transformation|SetWorldRotation (Variables|Default|GetSunDirectionalLight) (Math|Rotator|MakeRotator 0.0 (Math|Float|MapRangeUnclamped (Variables|01-BasicSettings|GetTimeOfDay) (- (Variables|01-BasicSettings|GetDawnTime) 0.3) (+ (Variables|01-BasicSettings|GetDuskTime) 0.3) 0.0 -1.8e+02) 0.0) false false)
  ;[0.15 0.15 0.15 0.5] Handle Moon rotation after dusk
  (Transformation|SetWorldRotation (Variables|Default|GetMoonDirectionalLight) (Math|Rotator|MakeRotator 0.0 (Math|Float|MapRangeUnclamped (Variables|01-BasicSettings|GetTimeOfDay) (+ (Variables|01-BasicSettings|GetDuskTime) 0.3) 24.0 0.0 -9e+01) 0.0) false false)
  ;[0.15 0.15 0.15 0.5] Handle Moon rotation before dawn
  (Transformation|SetWorldRotation (Variables|Default|GetMoonDirectionalLight) (Math|Rotator|MakeRotator 0.0 (Math|Float|MapRangeUnclamped (Variables|01-BasicSettings|GetTimeOfDay) 0.0 (- (Variables|01-BasicSettings|GetDawnTime) 0.3) -9e+01 -1.8e+02) 0.0) false false))

(fn HandleNightSettings
  (if (Utilities|IsNightTime) ; Night or Day?
    (Utilities|FlowControl|Sequence
      (:then_0
        ;[0.15 0.15 0.15 0.5] Moon Directional Light
        (Rendering|Components|Light|SetIntensity (Variables|Default|GetMoonDirectionalLight) (Variables|03-NightSettings|GetMoonlight%20Intensity))
        (Rendering|Components|Light|SetLightColor (Variables|Default|GetMoonDirectionalLight) (Variables|03-NightSettings|GetMoonlight%20Color) true)
        (Class|DirectionalLightComponent|SetLightSourceAngle (Variables|Default|GetMoonDirectionalLight) (Variables|03-NightSettings|GetMoonlight%20SourceAndle))
        (Class|LightComponent|SetTemperature (Variables|Default|GetMoonDirectionalLight) (Variables|03-NightSettings|GetMoonlight%20Temperature)))
      (:then_1
        ;[0.15 0.15 0.15 0.5] Sky Atmosphere
        (Class|SkyAtmosphereComponent|SetRayleighScattering (Variables|Default|GetSkyAtmosphere) (Variables|03-NightSettings|GetNightTime%20Rayleigh%20Scattering))
        (Class|SkyAtmosphereComponent|SetMultiScatteringFactor (Variables|Default|GetSkyAtmosphere) (Variables|03-NightSettings|GetNightTime%20MultiScattering)))
      (:then_2
        (Rendering|Material|SetScalarParameterValue (Variables|Default|GetCreated_DynMI_SkySphere) "IsStarVisible" (Math|Float|SelectFloat 1.0 0.0 (Variables|03-NightSettings|GetShouldShowNightStars)) :!class /Script/Engine.MaterialInstanceDynamic)
        (Rendering|Material|SetScalarParameterValue (Variables|Default|GetCreated_DynMI_SkySphere) "IsMoonVisible" (Math|Float|SelectFloat 1.0 0.0 (Variables|03-NightSettings|GetShouldShowMoon)) :!class /Script/Engine.MaterialInstanceDynamic)
        (Rendering|Material|SetVectorParameterValue (Variables|Default|GetCreated_DynMI_SkySphere) "MoonBasicSettings" (Utilities|Struct|MakeLinearColor (/ (Variables|03-NightSettings|GetMoon%20Scale) 1e+01) (Variables|03-NightSettings|GetMoon%20Rotation) (Variables|03-NightSettings|GetMoon%20Brightness) 1.0) :!class /Script/Engine.MaterialInstanceDynamic)
        (Rendering|Material|SetVectorParameterValue (Variables|Default|GetCreated_DynMI_SkySphere) "MoonTint" (Variables|03-NightSettings|GetMoon%20Tint) :!class /Script/Engine.MaterialInstanceDynamic)))
    (else
      ;[0.15 0.15 0.15 0.5] Sky Atmosphere
      (Class|SkyAtmosphereComponent|SetRayleighScattering (Variables|Default|GetSkyAtmosphere) (Variables|02-DaySettings|GetDayTime%20Rayleigh%20Scattering))
      (Class|SkyAtmosphereComponent|SetMultiScatteringFactor (Variables|Default|GetSkyAtmosphere) (Variables|02-DaySettings|GetDayTime%20Multi%20Scattering))
      (Rendering|Material|SetScalarParameterValue (Variables|Default|GetCreated_DynMI_SkySphere) "IsStarVisible" 0.0 :!class /Script/Engine.MaterialInstanceDynamic)
      (Rendering|Material|SetScalarParameterValue (Variables|Default|GetCreated_DynMI_SkySphere) "IsMoonVisible" 0.0 :!class /Script/Engine.MaterialInstanceDynamic))))